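; BP_MainGameMode is the game mode that runs the shared countdown timer for the puzzle game.
; Every Tick it calls DecreaseTime, which loops over all BP_MainPlayerState instances and maps each TimeDelation state to a normal, slow or fast rate.
; Each player subtracts an equal share of delta time, scaled by that rate, from RemainingTime on BP_MainGameState, so the clock follows the players' average rate.
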(event EventBeginPlay)

(event EventTick
  (params (DeltaSeconds :type Float%20%28single-precision%29))
  (CallFunction|DecreaseTime DeltaSeconds))

(fn ConstructionScript)

(fn DecreaseTime
  (params (DeltaTime :type Float%20%28double-precision%29))
  (for _index (range 0 (- (Class|GameplayStatics|GetNumPlayerStates) 1))
    (bind _asbp_main_player_state (Utilities|Casting|CastToBP_MainPlayerState (Game|GetPlayerState _index)))
    (switch Utilities|FlowControl|Switch|SwitchonENUM_TimeDelation (Variables|/Game/Puzzler/MainGameMode/BP_MainPlayerState.BP_MainPlayerState_C|GetTimeDelation _asbp_main_player_state)
      (:NewEnumerator2
        (LocalVariables|SetDelation 1.0))
      (:NewEnumerator0
        (LocalVariables|SetDelation (Variables|Default|GetSlowDelation)))
      (:NewEnumerator1
        (LocalVariables|SetDelation (Variables|Default|GetFastDelation))))
    (bind _asbp_main_game_state (Utilities|Casting|CastToBP_MainGameState (Game|GetGameState)))
    (Variables|/Game/Puzzler/MainGameMode/BP_MainGameState.BP_MainGameState_C|SetRemainingTime _asbp_main_game_state (- (Variables|/Game/Puzzler/MainGameMode/BP_MainGameState.BP_MainGameState_C|GetRemainingTime _asbp_main_game_state) (* (LocalVariables|GetDelation) (/ DeltaTime (Class|GameplayStatics|GetNumPlayerStates)))))))