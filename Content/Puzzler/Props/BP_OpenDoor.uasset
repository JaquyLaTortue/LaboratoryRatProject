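; Interactable puzzle door that opens once the player has collected all the cheese.
; Interact calls the parent, then, while the door is closed, compares NumberOfCheese with MaxCheese on player 0's BP_MainPlayerState.
; A match plays the OpenDoors sequence and clears DoorClosed, so the door opens only once.
; NewFunction repeats the cheese check but does nothing with the result, and the event graph is empty.
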(event EventBeginPlay)

(event Collision|EventActorBeginOverlap
  (params (OtherActor :type Actor%20Object%20Reference)))

(event EventTick
  (params (DeltaSeconds :type Float%20%28single-precision%29)))

(fn ConstructionScript)

(fn Interact
  (params (Character :type BP%20Main%20Character%20Object%20Reference))
  (|CallParentFunction Character)
  (if (Variables|Default|GetdoorClosed)
    (bind _asbp_main_player_state (Utilities|Casting|CastToBP_MainPlayerState (Game|GetPlayerState 0)))
    (if (== (Variables|/Game/Puzzler/MainGameMode/BP_MainPlayerState.BP_MainPlayerState_C|GetnumberOfCheese _asbp_main_player_state) (Variables|/Game/Puzzler/MainGameMode/BP_MainPlayerState.BP_MainPlayerState_C|GetMaxCheese _asbp_main_player_state))
      (Class|ActorSequenceComponent|PlaySequence (Variables|Default|GetOpenDoors))
      (Variables|Default|SetdoorClosed false))))

(fn NewFunction
  (bind _asbp_main_player_state (Utilities|Casting|CastToBP_MainPlayerState (Game|GetPlayerState 0)))
  (if (== (Variables|/Game/Puzzler/MainGameMode/BP_MainPlayerState.BP_MainPlayerState_C|GetMaxCheese _asbp_main_player_state) (Variables|/Game/Puzzler/MainGameMode/BP_MainPlayerState.BP_MainPlayerState_C|GetNumberOfCheese _asbp_main_player_state))
    _))