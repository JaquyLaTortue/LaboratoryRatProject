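; BP_elevator is an elevator prop that travels between a low and a high position, animated by sequences.
; Overlapping the inner Collision while the door is open closes it, moves the car up or down by toggling IsLow, then reopens it.
; Overlapping DoorCollision toggles the door open or closed.
; Fixed delays space the steps rather than sequence completion, and debug prints show the travel direction.
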(event OnComponentBeginOverlap(DoorCollision)
  (params (OverlappedComponent :type Primitive%20Component%20Object%20Reference) (OtherActor :type Actor%20Object%20Reference) (OtherComp :type Primitive%20Component%20Object%20Reference) (OtherBodyIndex :type Integer) (bFromSweep :type Boolean) (SweepResult :type Hit%20Result%20Structure%20%28by%20ref%29))
  (if (== (Variables|Default|GetDoorOpen) false)
    (Class|ActorSequenceComponent|PlaySequence (Variables|Default|GetOpenTheDoorSequence))
    (Utilities|FlowControl|Delay 5.0)
    (Variables|Default|SetDoorOpen true)
    (else
      (Class|ActorSequenceComponent|PlaySequence (Variables|Default|GetCloseTheDoorSequence))
      (Utilities|FlowControl|Delay 5.0)
      (Variables|Default|SetDoorOpen false))))

(event OnComponentBeginOverlap(Collision)
  (params (OverlappedComponent :type Primitive%20Component%20Object%20Reference) (OtherActor :type Actor%20Object%20Reference) (OtherComp :type Primitive%20Component%20Object%20Reference) (OtherBodyIndex :type Integer) (bFromSweep :type Boolean) (SweepResult :type Hit%20Result%20Structure%20%28by%20ref%29))
  (if (== (Variables|Default|GetDoorOpen) true)
    (Class|ActorSequenceComponent|PlaySequence (Variables|Default|GetCloseTheDoorSequence))
    (Utilities|FlowControl|Delay 5.0)
    (if (Variables|Default|GetIsLow)
      (Development|PrintString "UP")
      (Variables|Default|SetIsLow false)
      (Class|ActorSequenceComponent|PlaySequence (Variables|Default|GetElevatorUpSequence))
      (else
        (Development|PrintString "down")
        (Variables|Default|SetIsLow true)
        (Class|ActorSequenceComponent|PlaySequence (Variables|Default|GetElevatorLowSequence))))
    (Utilities|FlowControl|Delay 5.0)
    (Class|ActorSequenceComponent|PlaySequence (Variables|Default|GetOpenTheDoorSequence))
    (Utilities|FlowControl|Delay 5.0)
    (Variables|Default|SetDoorOpen true)))

(event EventBeginPlay)

(event EventTick
  (params (DeltaSeconds :type Float%20%28single-precision%29)))

(fn ConstructionScript)