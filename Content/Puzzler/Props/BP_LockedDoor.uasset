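; BP_LockedDoor is a puzzle door that opens when the player interacts while holding exactly as many keys as it has locks.
; Interact compares the key count in BP_MainPlayerState with the lock count, and CheckAndOpenDoor repeats that check before playing the door-opening sequence.
; On BeginPlay, a text label shows inserted keys over locks, green if equal, though this graph never updates the inserted count.
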(event EventBeginPlay
  (CallFunction|SetKeyText))

(event Collision|EventActorBeginOverlap
  (params (OtherActor :type Actor%20Object%20Reference))
  (|CallParentFunction OtherActor) ; This node is disabled and will not be called.\nDrag off pins to build functionality.
)

(event EventTick
  (params (DeltaSeconds :type Float%20%28single-precision%29)))

(fn ConstructionScript
  (|CallParentFunction))

(fn SetKeyText
  (Rendering|Components|TextRender|SetText (Variables|Default|GetKeyText) (Utilities|Text|FormatText "{keys} / {locks}" (Variables|Default|GetInstertedKeys) (Variables|Default|GetNumberOfLocks)))
  (if (== (Variables|Default|GetNumberOfLocks) (Variables|Default|GetInstertedKeys))
    (Rendering|Components|TextRender|SetTextRenderColor (Variables|Default|GetKeyText) (Math|Color|MakeColor 0 255 0))))

(fn Interact
  (params (Character :type BP%20Main%20Character%20Object%20Reference))
  (|CallParentFunction Character)
  (bind _asbp_main_player_state (Utilities|Casting|CastToBP_MainPlayerState (Game|GetPlayerState 0)))
  (if (== (Variables|/Game/Puzzler/MainGameMode/BP_MainPlayerState.BP_MainPlayerState_C|GetNumberOfKeys _asbp_main_player_state) (Variables|Default|GetNumberOfLocks))
    (CallFunction|CheckandOpenDoor)))

(fn CheckandOpenDoor
  (bind _asbp_main_player_state (Utilities|Casting|CastToBP_MainPlayerState (Game|GetPlayerState 0)))
  (if (== (Variables|Default|GetNumberOfLocks) (Variables|/Game/Puzzler/MainGameMode/BP_MainPlayerState.BP_MainPlayerState_C|GetNumberOfKeys _asbp_main_player_state))
    (Class|ActorSequenceComponent|PlaySequence (Variables|Default|GetOpenDoorSequence))))