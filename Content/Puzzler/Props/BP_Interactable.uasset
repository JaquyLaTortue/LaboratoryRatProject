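; BP_Interactable is a puzzle prop with an empty Interact function, apparently a base for interactable objects.
; On overlap with BP_MainCharacter, it registers itself as the character's CurrentInteractable and plays a ping sound.
; It then finds the pawn through the player controller and calls Interact immediately, passing no character.
; The section labeled for adding an informative widget creates no widget.
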(event Collision|EventActorBeginOverlap
  (params (OtherActor :type Actor%20Object%20Reference))
  ;[1 0.2645 0.7244 1 15] Register Interactable with Character
  (bind _asbp_main_character (Utilities|Casting|CastToBP_MainCharacter OtherActor))
  (Variables|/Game/Puzzler/MainGameMode/BP_MainCharacter.BP_MainCharacter_C|SetCurrentInteractable _asbp_main_character self)
  (Audio|PlaySound2D "/Game/Puzzler/Sounds/ping-82822.ping-82822" 1.0 1.0 0.0 0 0)
  ;[0.217 0.3564 1 1 15] Add Informative Widget to Viewport
  (bind _controller (CallFunction|GetPlayerController _asbp_main_character))
  (Utilities|IsValid _controller
    (:Is%20Valid
      (bind _asbp_main_character_2 (Utilities|Casting|CastToBP_MainCharacter (Pawn|GetControlledPawn _controller)))
      (Utilities|IsValid (Variables|/Game/Puzzler/MainGameMode/BP_MainCharacter.BP_MainCharacter_C|GetCurrentInteractable _asbp_main_character_2)
        (:Is%20Valid
          (CallFunction|Interact))))))

(fn ConstructionScript)

(fn Interact
  (params (Character :type BP%20Main%20Character%20Object%20Reference)))

(fn GetPlayerController
  (params (Actor :type Actor%20Object%20Reference))
  (bind _ascharacter (Utilities|Casting|CastToCharacter Actor))
  (bind _asplayer_controller (Utilities|Casting|CastToPlayerController (Pawn|GetController _ascharacter)))
  (return _asplayer_controller))