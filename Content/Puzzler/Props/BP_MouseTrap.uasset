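; BP_MouseTrap is a puzzle-game prop that kills the player when the main character touches it.
; On actor overlap it requires an exact BP_MainCharacter class match and an enabled CanBeActivate flag.
; It then clears the flag so it fires only once, plays the Activation sequence and calls Death on player 0's BP_MainPlayerController.
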(event EventBeginPlay)

(event Collision|EventActorBeginOverlap
  (params (OtherActor :type Actor%20Object%20Reference))
  (if (== (Utilities|GetClass OtherActor) "/Game/Puzzler/MainGameMode/BP_MainCharacter.BP_MainCharacter_C")
    (if (Variables|Default|GetcanBeActivate)
      (Variables|Default|SetcanBeActivate false)
      (Class|ActorSequenceComponent|PlaySequence (Variables|Default|GetActivation))
      (bind _asbp_main_player_controller (Utilities|Casting|CastToBP_MainPlayerController (Game|GetPlayerController 0)))
      (Default|Death _asbp_main_player_controller))))

(event EventTick
  (params (DeltaSeconds :type Float%20%28single-precision%29)))

(fn ConstructionScript)