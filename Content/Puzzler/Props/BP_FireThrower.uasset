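; BP_FireThrower is a puzzle-game prop that switches its fire particle effect on and off on a repeating cycle.
; Tick uses the WaitTheActivate flag as a latch around a fixed Delay, then calls ActiveTheFireThrower to flip the Active state and activate or deactivate the ParticleSystem.
; The file contains only this visual toggle, with no damage or overlap logic.
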(event EventBeginPlay)

(event Collision|EventActorBeginOverlap
  (params (OtherActor :type Actor%20Object%20Reference)))

(event EventTick
  (params (DeltaSeconds :type Float%20%28single-precision%29))
  (if (== (Variables|Default|GetwaitTheActivate) false)
    (Variables|Default|SetwaitTheActivate true)
    (Utilities|FlowControl|Delay 4.0)
    (CallFunction|ActivetheFireThrower)
    (Variables|Default|SetwaitTheActivate false)))

(fn ConstructionScript)

(fn ActivetheFireThrower
  (bind _particlesystem (Variables|Default|GetParticleSystem))
  (if (Variables|Default|Getactive)
    (Components|Activation|Deactivate _particlesystem)
    (Variables|Default|Setactive false)
    (else
      (Components|Activation|Activate _particlesystem false)
      (Variables|Default|Setactive true))))